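; Fire effect actor that lets DMX lighting data drive the spawn rate of its Niagara particle system.
; On BeginPlay it subscribes to the DMX subsystem's protocol-received event, and the DMX component's fixture-patch-received event feeds the same update.
; That update reads an attribute value from the component's fixture patch, scales it down by a constant and writes it to the Niagara SpawnRate variable.
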(event OnFixturePatchReceived(DMX)
  (params (FixturePatch :type DMX%20Entity%20Fixture%20Patch%20Object%20Reference) (ValuePerAttribute :type DMX%20Normalized%20Attribute%20Value%20Map%20Structure%20%28by%20ref%29))
  (bind _outattributesmap (|GetDMXAttributeValues (Class|DMXComponent|GetFixturePatch (Variables|Default|GetDMX))))
  (Niagara|SetNiagaraVariable(Float) (Variables|NiagaraActor|GetNiagaraComponent) "SpawnRate" (/ (Math|Conversions|ToFloat(Integer) (.Value (Utilities|Map|Find _outattributesmap "(Name=\"Dimmer\")"))) 2.8)))

(event Custom|OnProtocolReceived_Event_0
  (params (Protocol :type DMX%20Protocol%20Name%20Structure) (RemoteUniverse :type Integer) (DMXBuffer :type Array%20of%20Bytes))
  (bind _outattributesmap (|GetDMXAttributeValues (Class|DMXComponent|GetFixturePatch (Variables|Default|GetDMX))))
  (Niagara|SetNiagaraVariable(Float) (Variables|NiagaraActor|GetNiagaraComponent) "SpawnRate" (/ (Math|Conversions|ToFloat(Integer) (.Value (Utilities|Map|Find _outattributesmap "(Name=\"Dimmer\")"))) 2.8)))

(event EventBeginPlay
  (EventDispatchers|AssignOnProtocolReceived (|DMXSubsystem) (delegate Custom|OnProtocolReceived_Event_0)))

(event EventTick
  (params (DeltaSeconds :type Float%20%28single-precision%29)))

(fn ConstructionScript)