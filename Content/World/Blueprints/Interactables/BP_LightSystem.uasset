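; BP_LightSystem is an interactable that lets a player take control of lighting.
; It binds to an interact event on BeginPlay and accepts an interacting player only while its RepNotify Player variable is unset; the OnRep is empty.
; It then calls ModifyLighting on that player's BP_CharacterController, passing its Arrow component's world transform as the spawn transform along with the player.
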(event Custom|Interacted
  (params (Player :type BP%20Character%20Object%20Reference))
  (Utilities|IsValid (Variables|Default|GetPlayer)
    (:Is%20Not%20Valid
      (bind _output_get (Variables|Default|SetPlayer Player))
      (CallFunction|EnableLightingControls _output_get))))

(event EventBeginPlay
  (EventDispatchers|BindEventtoInteract (delegate Custom|Interacted)))

(fn ConstructionScript
  (|CallParentFunction))

(fn OnRepPlayer)

(fn EnableLightingControls
  (params (Player :type BP%20Character%20Object%20Reference))
  (bind _asbp_character_controller (Utilities|Casting|CastToBP_CharacterController (Pawn|GetController Player)))
  (Default|ModifyLighting _asbp_character_controller (Transformation|GetWorldTransform (Variables|Default|GetArrow)) Player))