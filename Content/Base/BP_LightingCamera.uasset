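; BP_LightingCamera is a player-controlled camera Blueprint that opens the UI_Lighting widget for its local player.
; LookUp and Turn axis inputs drive controller pitch and yaw.
; On BeginPlay, outside dedicated servers, it creates the widget and switches UI mode with the mouse shown.
; An IsLocalClient check compares the owner to player controller 0, so the screen is not duplicated.
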(event EventBeginPlay
  (if (not (Networking|IsDedicatedServer))
    (if (CallFunction|IsLocalClient)
      (bind _returnvalue (UserInterface|CreateWidget "/Game/Interface/UI_Lighting.UI_Lighting_C"))
      (UserInterface|Viewport|AddtoViewport _returnvalue 0)
      (CallFunction|SetUIMode "NewEnumerator2" true))))

(event Input|AxisEvents|InputAxisLookUp
  (params (AxisValue :type Float%20%28single-precision%29))
  (Pawn|Input|AddControllerPitchInput AxisValue))

(event Input|AxisEvents|InputAxisTurn
  (params (AxisValue :type Float%20%28single-precision%29))
  (Pawn|Input|AddControllerYawInput AxisValue))

(fn ConstructionScript)

(fn IsLocalClient
  (return (== (Components|GetOwner) (Game|GetPlayerController 0))))